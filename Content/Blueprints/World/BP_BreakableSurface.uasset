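; Diggable surface actor built on a dynamic mesh that can have holes carved into it at runtime.
; The construction script rebuilds it as a collision box from the SurfaceDimension variables.
; DigHole boolean-subtracts a squashed sphere from a pooled compute mesh, flattened in Z for up/down digs or in X otherwise.
; Hole placement subtracts only the actor's location, ignoring its rotation and scale.
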(event `DigHole`
  (params (HoleLocation :type "Vector Structure") (isDown :type Boolean) (isUp :type Boolean))
  ; DigHole Event
  (bind _returnvalue (`self.AllocateComputeMesh`))
  (if isDown
    ;;[0.09492 0 0.15 0.5] Up&Down Dig Scale
    (bind _returnvalue_2 (`GeometryScriptLibrary_MeshPrimitiveFunctions.AppendSphereBox` _returnvalue (struct) (`KismetMathLibrary.MakeTransform` (- HoleLocation (`self.K2_GetActorLocation`)) (struct) (1.5 1.5 0.5)) 100.0 6 6 6 "Center" null :!label _label))
    (bind _returnvalue_3 (`BaseDynamicMeshComponent.GetDynamicMesh` (`self.DynamicMeshComponent`)))
    (`GeometryScriptLibrary_MeshBooleanFunctions.ApplyMeshBoolean` _returnvalue_3 (struct) _returnvalue_2 (struct) "Subtract" (struct) null)
    (`self.ReleaseAllComputeMeshes`)
    (elif isUp
      (goto _label)
      (else
        ;;[0.09492 0 0.15 0.5] Face Dig Scale
        (bind _returnvalue_4 (`GeometryScriptLibrary_MeshPrimitiveFunctions.AppendSphereBox` _returnvalue (struct) (`KismetMathLibrary.MakeTransform` (- HoleLocation (`self.K2_GetActorLocation`)) (struct) (0.75 1.5 1.5)) 100.0 6 6 6 "Center" null))
        (bind _returnvalue_5 (`BaseDynamicMeshComponent.GetDynamicMesh` (`self.DynamicMeshComponent`)))
        (`GeometryScriptLibrary_MeshBooleanFunctions.ApplyMeshBoolean` _returnvalue_5 (struct) _returnvalue_4 (struct) "Subtract" (struct) null)
        (`self.ReleaseAllComputeMeshes`)))))

(fn `UserConstructionScript`
  (bind _returnvalue (`BaseDynamicMeshComponent.GetDynamicMesh` (`self.DynamicMeshComponent`)))
  (bind _returnvalue_2 (`DynamicMesh.Reset` _returnvalue))
  (`GeometryScriptLibrary_MeshPrimitiveFunctions.AppendBoxWithCollision` _returnvalue_2 (struct) (struct) (`self.SurfaceDimensionX`) (`self.SurfaceDimensionY`) (`self.SurfaceDimensionZ`) 0 0 0 "Base" null))